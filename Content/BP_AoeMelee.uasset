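; BP_AoeMelee is a melee area-of-effect combo attack for the player in combat.
; Enemy overlaps toggle their target flag and the combat menu's combo button.
; CastAoe plays one of three montages by combo count, switching input contexts around them; notifies damage all overlapped enemies through the combat system.
; The count increments per enemy hit, wrapping at the maximum and increasing the participant's action count.
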(event `self.ReceiveBeginPlay`
  (set `self.MaxComboCount` 3)
  (set `self.CurrentComboCount` 0)
  (bind _asbp_third_person_character (cast `/Game/ThirdPerson/Blueprints/BP_ThirdPersonCharacter` (`Controller.K2_GetPawn` (`GameplayStatics.GetPlayerController` 0))))
  (set `self.CharacterMesh` (`Character.Mesh` _asbp_third_person_character)))

(event `self.ReceiveActorBeginOverlap`
  (params (OtherActor :type "Actor Object Reference"))
  (bind _asbp_enemy_character (cast `/Game/ThirdPerson/Blueprints/BP_EnemyCharacter` OtherActor))
  (set `/Game/ThirdPerson/Blueprints/BP_EnemyCharacter.IsTarget` true _asbp_enemy_character)
  ;[1 1 1] TODO: getting widgets every time is wasteful. Come tighten this up later
  (bind _foundwidgets (`WidgetBlueprintLibrary.GetAllWidgetsOfClass` "/Game/ThirdPerson/Blueprints/BP_CombatMenuWidget.BP_CombatMenuWidget_C"))
  (for _array_element _foundwidgets
    (set `Widget.Visibility` "Visible" (`/Game/ThirdPerson/Blueprints/BP_CombatMenuWidget.ComboButton` _array_element))))

(event `self.ReceiveActorEndOverlap`
  (params (OtherActor :type "Actor Object Reference"))
  (bind _asbp_enemy_character (cast `/Game/ThirdPerson/Blueprints/BP_EnemyCharacter` OtherActor))
  (set `/Game/ThirdPerson/Blueprints/BP_EnemyCharacter.IsTarget` false _asbp_enemy_character)
  ;[1 1 1] TODO: getting widgets every time is wasteful. Come tighten this up later
  (bind _foundwidgets (`WidgetBlueprintLibrary.GetAllWidgetsOfClass` "/Game/ThirdPerson/Blueprints/BP_CombatMenuWidget.BP_CombatMenuWidget_C"))
  (for _array_element _foundwidgets
    (set `Widget.Visibility` "Hidden" (`/Game/ThirdPerson/Blueprints/BP_CombatMenuWidget.ComboButton` _array_element))))

(event `self.CastAoe`
  (bind _charactermesh (`self.CharacterMesh`))
  (if (> (`KismetArrayLibrary.Array_Length` (`self.GetOverlappingActors` "/Game/ThirdPerson/Blueprints/BP_EnemyCharacter.BP_EnemyCharacter_C")) 0)
    (bind _asbp_player_controller (cast `/Game/ThirdPerson/Blueprints/BP_PlayerController` (`GameplayStatics.GetPlayerController` 0)))
    (`MyPlayerController.SwitchInputMappingContext` _asbp_player_controller "/Game/ThirdPerson/Input/Combat/IMC_CameraOnly.IMC_CameraOnly")
    (switch `int` (`self.CurrentComboCount`)
      (:`0`
        (`|PlayMontage` _charactermesh "/Game/Guild/Characters/Mike/Mike_Combo_1.Mike_Combo_1"
          (:`OnNotifyBegin`
            (for _array_element (`self.GetOverlappingActors` "/Game/ThirdPerson/Blueprints/BP_EnemyCharacter.BP_EnemyCharacter_C") :!label _label
              (`CombatSystem.ApplyDamage` (subsystem `CombatSystem`) 5 _array_element)
              (bind _result (`/Engine/EditorBlueprintResources/StandardMacros.IncrementInt` (`self.CurrentComboCount`))
                (:`  `
                  (bind _output_get (set `self.CurrentComboCount` _result))
                  (if (>= _output_get (`self.MaxComboCount`))
                    (set `self.CurrentComboCount` 0)
                    (`CombatSystem.InceaseCurrentParticipantActionCount` (subsystem `CombatSystem`)))))))
          (:`OnNotifyEnd`
            (bind _asbp_player_controller_2 (cast `/Game/ThirdPerson/Blueprints/BP_PlayerController` (`GameplayStatics.GetPlayerController` 0) :!label _label_2))
            (`MyPlayerController.SwitchInputMappingContext` _asbp_player_controller_2 "/Game/ThirdPerson/Input/Combat/IMC_Combo.IMC_Combo"))))
      (:`1`
        (`|PlayMontage` _charactermesh "/Game/Guild/Characters/Mike/Mike_Combo_2.Mike_Combo_2"
          (:`OnNotifyBegin`
            (goto _label))
          (:`OnNotifyEnd`
            (goto _label_2))))
      (:`2`
        (`|PlayMontage` _charactermesh "/Game/Guild/Characters/Mike/Mike_Combo_3.Mike_Combo_3"
          (:`OnNotifyBegin`
            (goto _label))
          (:`OnNotifyEnd`
            (bind _asbp_player_controller_3 (cast `/Game/ThirdPerson/Blueprints/BP_PlayerController` (`GameplayStatics.GetPlayerController` 0)))
            (`MyPlayerController.SetCombatInput` _asbp_player_controller_3)))))))

(fn `UserConstructionScript`)