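; BP_AoeDirect is a directional area-of-effect targeting actor that marks the enemies inside its overlap area.
; Begin and end overlap toggle IsTarget on each BP_EnemyCharacter, while Tick draws a debug arrow along the actor's forward vector.
; CastAoe only calls StopInput on the player controller; a Cleave montage node is present but never runs, and no damage is applied here.
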(event `self.ReceiveTick`
  (params (DeltaSeconds :type "Float (single-precision)"))
  (bind _returnvalue (`self.K2_GetActorLocation`))
  (`KismetSystemLibrary.DrawDebugArrow` _returnvalue (+ _returnvalue (* (`self.GetActorForwardVector`) 160)) 50.0 (struct :`R` 1.0 :`G` 0.215227 :`B` 0.939596 :`A` 1.0) 0.0 3.0))

(event `self.ReceiveActorBeginOverlap`
  (params (OtherActor :type "Actor Object Reference"))
  (bind _asbp_enemy_character (cast `/Game/ThirdPerson/Blueprints/BP_EnemyCharacter` OtherActor))
  (set `/Game/ThirdPerson/Blueprints/BP_EnemyCharacter.IsTarget` true _asbp_enemy_character))

(event `self.ReceiveActorEndOverlap`
  (params (OtherActor :type "Actor Object Reference"))
  (bind _asbp_enemy_character (cast `/Game/ThirdPerson/Blueprints/BP_EnemyCharacter` OtherActor))
  (set `/Game/ThirdPerson/Blueprints/BP_EnemyCharacter.IsTarget` false _asbp_enemy_character))

(event `self.CastAoe`
  (bind _asbp_player_controller (cast `/Game/ThirdPerson/Blueprints/BP_PlayerController` (`GameplayStatics.GetPlayerController` 0)))
  (`MyPlayerController.StopInput` _asbp_player_controller))

(fn `UserConstructionScript`)