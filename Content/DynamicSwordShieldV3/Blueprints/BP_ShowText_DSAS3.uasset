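; Labels the SkeletalMeshActors in the level with animation names, apparently for a sword and shield animation showcase.
; ShowTexts, run from the construction script and BeginPlay, loops over those actors and adds an offset, centered TextRenderComponent to each.
; The label is the actor display name after the AnimTitle substring, left blank if it contains Run or Walk.
; TextScale and TextColor set its appearance.
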(event `AddTextComponent`
  (params (SkeletalMeshActor :type "Actor Object Reference"))
  (bind _textscale (`self.TextScale`))
  (bind (_lefts _rights) (`KismetStringLibrary.Split` (`KismetSystemLibrary.GetDisplayName` SkeletalMeshActor) (`self.AnimTitle`)))
  ;[1 1 1] Add text component
  (bind _returnvalue (`|AddComponentByClass` SkeletalMeshActor "/Script/Engine.TextRenderComponent" false (`KismetMathLibrary.MakeTransform` (0.0 120.0 0.0) (struct :`Pitch` 45.0 :`Yaw` 90.0))))
  (`TextRenderComponent.K2_SetText` _returnvalue (`KismetTextLibrary.Conv_StringToText` (select `bool` (or (`KismetStringLibrary.Contains` _rights "Run") (`KismetStringLibrary.Contains` _rights "Walk")) :`false` _rights)))
  (`TextRenderComponent.SetXScale` _returnvalue _textscale)
  (`TextRenderComponent.SetYScale` _returnvalue _textscale)
  (`TextRenderComponent.SetTextRenderColor` _returnvalue (`self.TextColor`))
  (`TextRenderComponent.SetHorizontalAlignment` _returnvalue "EHTA_Center"))

(event `self.ReceiveBeginPlay`
  ;[1 1 1] Add text component
  (`self.ShowTexts`))

(fn `ShowTexts`
  (bind _outactors (`GameplayStatics.GetAllActorsOfClass` "/Script/Engine.SkeletalMeshActor"))
  (if (`KismetArrayLibrary.Array_IsValidIndex` _outactors)
    (for _array_element _outactors
      (`/Engine/EditorBlueprintResources/StandardMacros.IsValid` _array_element
        (:`Is Valid`
          (`self.AddTextComponent` _array_element))))))

(fn `UserConstructionScript`
  (`self.ShowTexts`))